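; Controller for the UFO pawn that flies it along a looping spline path while spinning it.
; On BeginPlay it caches the possessed UFO and the spline component of the Spline_UFO actor found in the level.
; Each Tick it advances distance by the UFO's Velocity, wrapping at a hardcoded length rather than the spline's.
; It then moves the UFO to that world-space point and applies local pitch and yaw rotation.
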(event EventBeginPlay
  (bind _asufo (Utilities|Casting|CastToUFO (Pawn|GetControlledPawn)))
  (Variables|Default|SetUFO _asufo)
  (bind _returnvalue (Actor|GetActorOfClass "/Game/Blueprints/Spline_UFO.Spline_UFO_C"))
  (Variables|Default|Setspline_ufo (Actor|GetComponentbyClass _returnvalue "/Script/Engine.SplineComponent")))

(event EventTick
  (params (DeltaSeconds :type Float%20%28single-precision%29))
  (bind _ufo (Variables|Default|GetUFO))
  (bind _speed_rotate (Variables|Default|Getspeed_rotate))
  (bind _returnvalue (* DeltaSeconds _speed_rotate))
  (bind _output_get (Variables|Default|Setdistance (+ (Variables|Default|Getdistance) (* DeltaSeconds (Variables|/Game/Blueprints/UFO.UFO_C|Getvelocity _ufo)))))
  (Variables|Default|Setdistance (Math|Float|%(Float) _output_get 8e+03))
  (Transformation|SetActorLocation _ufo (Spline|GetLocationatDistanceAlongSpline (Variables|Default|Getspline_ufo) _output_get "World") false false)
  (Transformation|AddActorLocalRotation _ufo (Math|Rotator|MakeRotator 0.0 _returnvalue _returnvalue) false false))

(fn ConstructionScript)