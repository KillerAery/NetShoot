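; Thrown bomb actor that launches its mesh forward on BeginPlay and damages nearby players when it explodes.
; It detonates on hitting a Shooter_Character or when Tick finds its squared speed below a threshold.
; Detonation distance-checks player indices 0 and 1, applying damage credited to the Shooter's controller.
; Flags let the next Tick spawn explosion effects and sound once, while a short timer destroys the actor.
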(event Custom|ApplyBoomAtPlayer
  (params (PlayerID :type Integer))
  (bind _returnvalue (Game|Player|GetPlayerPawn PlayerID))
  (Math|Float|CompareFloat (Class|KismetMathLibrary|VectorDistanceSquared (Transformation|GetWorldLocation (Variables|Default|GetBombMesh)) (Transformation|GetActorLocation _returnvalue)) 1e+05
    (:>
      (Development|PrintString "没有被BOOM波及"))
    (:<
      (bind _asshooter_character (Utilities|Casting|CastToShooter_Character (Variables|Default|GetShooter)))
      (Game|Damage|ApplyDamage _returnvalue 1e+02 (Pawn|GetController _asshooter_character) self)
      (Development|PrintString "Boom Damge Player"))))

(event Custom|DestoryBomb
  (Actor|DestroyActor))

(event EventTick
  (params (DeltaSeconds :type Float%20%28single-precision%29))
  (bind _bombmesh (Variables|Default|GetBombMesh))
  (bind _returnvalue (Transformation|GetWorldLocation _bombmesh))
  (if (Variables|Default|GetTesting)
    (Math|Float|CompareFloat (Math|Vector|VectorLengthSquared (Transformation|GetComponentVelocity (Variables|Default|GetBombMesh))) 8e+02
      (:<
        (Variables|Default|SetExplosed true)
        (Variables|Default|SetTesting false)
        (CallFunction|ApplyBoomatPlayer)
        (CallFunction|ApplyBoomatPlayer 1)
        (Development|PrintString "SERVER TRICK BOOM")
        (Utilities|Time|SetTimerbyEvent (delegate Custom|DestoryBomb) 0.5)))
    (elif (Variables|Default|GetExplosed)
      (Variables|Default|SetExplosed false)
      (Effects|SpawnEmitteratLocation "/Game/M5VFXVOL2/Particles/Explosion/Fire_Exp_00.Fire_Exp_00" _returnvalue)
      (Audio|PlaySoundatLocation "/Game/Sounds/BOOM.BOOM" _returnvalue "0, 0, 0" 1.0 1.0 0.0 0 0 0))))

(event Collision|EventHit
  (params (MyComp :type Primitive%20Component%20Object%20Reference) (Other :type Actor%20Object%20Reference) (OtherComp :type Primitive%20Component%20Object%20Reference) (bSelfMoved :type Boolean) (HitLocation :type Vector :default "0, 0, 0") (HitNormal :type Vector :default "0, 0, 0") (NormalImpulse :type Vector :default "0, 0, 0") (Hit :type Hit%20Result%20Structure%20%28by%20ref%29))
  (if (Variables|Default|GetTesting)
    (Utilities|Casting|CastToShooter_Character Other)
    (Variables|Default|SetExplosed true)
    (Variables|Default|SetTesting false)
    (CallFunction|ApplyBoomatPlayer)
    (CallFunction|ApplyBoomatPlayer 1)
    (Development|PrintString "SERVER TRICK BOOM")
    (Utilities|Time|SetTimerbyEvent (delegate Custom|DestoryBomb) 0.5)))

(event EventBeginPlay
  (bind _bombmesh (Variables|Default|GetBombMesh))
  (bind _returnvalue (Math|Vector|GetForwardVector _bombmesh))
  (Physics|AddImpulse (Variables|Default|GetBombMesh) (* _returnvalue (Variables|Default|Getimpluse)) "None" true)
  (Physics|SetPhysicsLinearVelocity (Variables|Default|GetBombMesh) (* _returnvalue 3e+01) false "None")
  (Variables|Default|SetTesting true))

(fn ConstructionScript)