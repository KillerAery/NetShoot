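; Behavior tree task that makes an AI character fire at the player.
; It reads the Player object from the blackboard and casts it to Shooter_Character, failing the task if it is missing or another type.
; It then sets the AI_Character's LookAt to the player's location, calls Firing and finishes with success.
; If the controlled pawn is not an AI_Character, the task stops without finishing.
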(event EventReceiveExecuteAI
  (params (OwnerController :type AI%20Controller%20Object%20Reference) (ControlledPawn :type Pawn%20Object%20Reference))
  (bind _returnvalue (Utilities|Name|MakeLiteralName "Player"))
  (bind _returnvalue_2 (Class|BTFunctionLibrary|GetOwnersBlackboard))
  (bind _returnvalue_3 (AI|Components|Blackboard|GetValueasObject _returnvalue_2 _returnvalue))
  (if (Utilities|IsValid _returnvalue_3)
    (bind _asshooter_character (Utilities|Casting|CastToShooter_Character _returnvalue_3)
      (:then
        (bind _asai_character (Utilities|Casting|CastToAI_Character ControlledPawn))
        (Variables|/Game/Blueprints/Shooter_Character.Shooter_Character_C|SetLookAt _asai_character (Transformation|GetActorLocation _asshooter_character))
        (Default|Firing _asai_character)
        (AI|BehaviorTree|FinishExecute true))
      (:CastFailed
        (AI|BehaviorTree|FinishExecute false :!label _label)))
    (else
      (goto _label))))