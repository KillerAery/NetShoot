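; Game state for a multiplayer timed match that tracks the countdown and a ranked leaderboard.
; On BeginPlay, the server loads ranks from the game mode's save game into RankMap and the name and score arrays meant for client sync.
; Tick starts the one-minute timer once two players join, then ends the match through player controller 0 at zero.
; Score changes update RankMap, then rebuild both arrays via UpdateDataByRankMap.
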(event EventBeginPlay
  ;[1 1 1] 服务器RankList同步到各个客户端
  (if (Networking|IsServer)
    (bind _asmy_game_mode (Utilities|Casting|CastToMyGameMode (Game|GetGameMode)))
    (for (_array_element _array_index) (Class|RankListSaveGame|GetRankListScore (Variables|/Game/Blueprints/MyGameMode.MyGameMode_C|GetRankListSaveGame _asmy_game_mode))
      (Utilities|Map|Add (Variables|Default|GetRankMap) (Utilities|Array|Get(acopy) (Class|RankListSaveGame|GetRankListName (Variables|/Game/Blueprints/MyGameMode.MyGameMode_C|GetRankListSaveGame _asmy_game_mode)) _array_index) _array_element))
    (Variables|Default|SetRankListScore (Class|RankListSaveGame|GetRankListScore (Variables|/Game/Blueprints/MyGameMode.MyGameMode_C|GetRankListSaveGame _asmy_game_mode)))
    (Variables|Default|SetRankListName (Class|RankListSaveGame|GetRankListName (Variables|/Game/Blueprints/MyGameMode.MyGameMode_C|GetRankListSaveGame _asmy_game_mode)))
    (Development|PrintString "Server Load RankList Done!")))

(event EventTick
  (params (DeltaSeconds :type Float%20%28single-precision%29))
  ;[1 1 1] Timer
  (if (not (Variables|Default|GetGameOver))
    (if (Variables|Default|GetGameStart)
      (bind _output_get (Variables|Default|Settimer (- (Variables|Default|Gettimer) DeltaSeconds)))
      ;[1 1 1] GameEnd
      (Math|Float|CompareFloat _output_get 0.0
        (:<
          (Variables|Default|Settimer 0.0)
          (Variables|Default|SetGameStart false)
          (Variables|Default|SetGameOver true)
          (bind _asmy_player_controller (Utilities|Casting|CastToMyPlayerController (Game|GetPlayerController 0)))
          (Default|GameOver _asmy_player_controller)))
      (else
        (Math|Integer|CompareInt (Variables|Default|GetPlayerNum) 2
          (:>
            _)
          (:==
            _))
        (CallFunction|StartTimer)))))

(fn ConstructionScript)

(fn StartTimer
  (Variables|Default|SetTimer 6e+01)
  (Variables|Default|SetGameStart true))

(fn ChangePlayerScore
  (params (PlayerName :type String) (DeltaScore :type Integer))
  (bind _rankmap (Variables|Default|GetRankMap))
  (bind _rankmap_2 (Variables|Default|GetRankMap))
  (bind (_value _returnvalue) (Utilities|Map|Find _rankmap_2 PlayerName))
  (if _returnvalue
    (Utilities|Map|Add _rankmap PlayerName (+ _value DeltaScore))
    (else
      (Utilities|Map|Add _rankmap PlayerName DeltaScore)))
  (CallFunction|UpdateRankList)
  (Development|PrintString "GameState:Change Score OK"))

(fn UpdateRankList
  (bind (_rankscore _rankname) (Class|RankListSaveGame|UpdateDatabyRankMap (Variables|Default|GetRankMap)))
  (Variables|Default|SetRankListScore _rankscore)
  (Variables|Default|SetRankListName _rankname))

(fn OnRepRankListScore)

(fn OnRepRankListName)

(fn OnRepChanged)